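; BP_Enemy is a Venus flytrap enemy that shoots and damages the Rogue player.
; Pawn sensing turns it toward a seen Rogue, then it plays an attack animation, spawns a projectile and applies damage directly, gated by a short cooldown.
; DamageBox hurts the Rogue when overlap ends, then makes a delayed damage call with no target.
; Taking damage lowers clamped health and plays hit feedback, destroying the actor at zero.
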(event OnSeePawn(PawnSensing)
  (params (Pawn :type Pawn%20Object%20Reference))
  ;[1 0 0.8744] Enemy shooting out character when in radius
  (bind _asrogue (Utilities|Casting|CastToRogue Pawn))
  (Transformation|SetActorRotation (Math|Rotator|FindRelativeLookatRotation (Math|Conversions|ToTransform(Vector) (Transformation|GetActorLocation)) (Transformation|GetActorLocation _asrogue)))
  (if (Variables|Default|GetCanAttack)
    (Components|Animation|PlayAnimation (Variables|Character|GetMesh) "/Game/Enemy/Animations/VenusFlyTrapAttack_Enemy_Anim.VenusFlyTrapAttack_Enemy_Anim" false)
    (Game|SpawnActorfromClass "/Game/Nadja/BP_FirstPersonProjectile.BP_FirstPersonProjectile_C" (Transformation|GetWorldTransform (Variables|Default|GetSpawnProjectileLocation)) "Undefined" 0 0)
    (Game|Damage|ApplyDamage _asrogue 1.0 0 0)
    (Variables|Default|SetCanAttack false)
    (Utilities|FlowControl|Delay 1.0)
    (Variables|Default|SetCanAttack true)))

(event OnComponentEndOverlap(DamageBox)
  (params (OverlappedComponent :type Primitive%20Component%20Object%20Reference) (OtherActor :type Actor%20Object%20Reference) (OtherComp :type Primitive%20Component%20Object%20Reference) (OtherBodyIndex :type Integer))
  ;[1 0.5 0.5 0.5] Can Damage Player
  (bind _asrogue (Utilities|Casting|CastToRogue OtherActor))
  (Game|Damage|ApplyDamage _asrogue 1.0 0 self)
  (Utilities|FlowControl|Delay 2.0)
  (Game|Damage|ApplyDamage 0 1.0 0 self))

(event Game|Damage|EventAnyDamage
  (params (Damage :type Float%20%28single-precision%29) (DamageType :type Damage%20Type%20Object%20Reference) (InstigatedBy :type Controller%20Object%20Reference) (DamageCauser :type Actor%20Object%20Reference))
  (bind _returnvalue (Transformation|GetActorLocation))
  ;[1 0.5 0.5 0.5] Enemy HP and Damage System
  (bind _output_get (Variables|Default|SetHealth (Math|Float|Clamp(Float) (- (Variables|Default|GetHealth) Damage) 0.0 5.0)))
  (if (== _output_get 0.0)
    (Audio|PlaySoundatLocation "/Game/Nadja/394466__plasterbrain__enemy-destroyed.394466__plasterbrain__enemy-destroyed" _returnvalue "0, 0, 0" 1.0 1.0 0.0 0 0 0 0)
    (Components|Animation|PlayAnimation (Variables|Character|GetMesh) "/Game/Enemy/Animations/VenusFlyTrapHit_Enemy_Anim.VenusFlyTrapHit_Enemy_Anim" false)
    (Actor|DestroyActor)
    (else
      (Audio|PlaySoundatLocation 0 _returnvalue "0, 0, 0" 1.0 1.0 0.0 0 0 0 0)
      (Components|Animation|PlayAnimation (Variables|Character|GetMesh) "/Game/Enemy/Animations/VenusFlyTrapHit_Enemy_Anim.VenusFlyTrapHit_Enemy_Anim" false))))

(event EventTick
  (params (DeltaSeconds :type Float%20%28single-precision%29))
  ;[1 0.5 0.5 0.5] Making Player a Variable
  (bind _asrogue (Utilities|Casting|CastToRogue (Game|GetPlayerCharacter 0)))
  (Variables|Default|SetAs%20Rogue _asrogue))

(fn ConstructionScript)