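; BP_DialogueTrigger is a trigger actor that shows monologue text on the tutorial HUD when the Rogue enters its Box volume.
; Entering Box sets the HUD's TxtMonologue to the Monologue variable and hides the Widget component; leaving clears the text and shows the widget again.
; A separate IconBox volume shows the widget on begin overlap and hides it on end overlap, without filtering by actor type.
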(event OnComponentBeginOverlap(IconBox)
  (params (OverlappedComponent :type Primitive%20Component%20Object%20Reference) (OtherActor :type Actor%20Object%20Reference) (OtherComp :type Primitive%20Component%20Object%20Reference) (OtherBodyIndex :type Integer) (bFromSweep :type Boolean) (SweepResult :type Hit%20Result%20Structure%20%28by%20ref%29))
  (Rendering|SetVisibility (Variables|Default|GetWidget) true false))

(event OnComponentBeginOverlap(Box)
  (params (OverlappedComponent :type Primitive%20Component%20Object%20Reference) (OtherActor :type Actor%20Object%20Reference) (OtherComp :type Primitive%20Component%20Object%20Reference) (OtherBodyIndex :type Integer) (bFromSweep :type Boolean) (SweepResult :type Hit%20Result%20Structure%20%28by%20ref%29))
  (bind _asrogue (Utilities|Casting|CastToRogue OtherActor))
  (Rendering|Components|TextRender|SetText (Variables|/Game/Renea/WBP_TutorialInfo.WBP_TutorialInfo_C|GetTxt_Monologue (Variables|/Game/Rogue2/Rogue.Rogue_C|GetTutorialHUD _asrogue)) (Variables|Default|GetMonologue))
  (Rendering|SetVisibility (Variables|Default|GetWidget) false false))

(event OnComponentEndOverlap(IconBox)
  (params (OverlappedComponent :type Primitive%20Component%20Object%20Reference) (OtherActor :type Actor%20Object%20Reference) (OtherComp :type Primitive%20Component%20Object%20Reference) (OtherBodyIndex :type Integer))
  (Rendering|SetVisibility (Variables|Default|GetWidget) false false))

(event OnComponentEndOverlap(Box)
  (params (OverlappedComponent :type Primitive%20Component%20Object%20Reference) (OtherActor :type Actor%20Object%20Reference) (OtherComp :type Primitive%20Component%20Object%20Reference) (OtherBodyIndex :type Integer))
  (bind _asrogue (Utilities|Casting|CastToRogue OtherActor))
  (Rendering|Components|TextRender|SetText (Variables|/Game/Renea/WBP_TutorialInfo.WBP_TutorialInfo_C|GetTxt_Monologue (Variables|/Game/Rogue2/Rogue.Rogue_C|GetTutorialHUD _asrogue)) "")
  (Rendering|SetVisibility (Variables|Default|GetWidget) true false))

(fn ConstructionScript)