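; BP_ArmorPiece is an armor pickup actor that represents a pendant, tiara or bracelet.
; The construction script picks the static mesh from the ArmorPiece value.
; A sphere overlap shows and hides its widget, with no filter on the overlapping actor.
; EquipPickUp returns the piece type to the caller and triggers PickedUp, which destroys the actor after a short delay.
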(event OnComponentBeginOverlap(Sphere)
  (params (OverlappedComponent :type Primitive%20Component%20Object%20Reference) (OtherActor :type Actor%20Object%20Reference) (OtherComp :type Primitive%20Component%20Object%20Reference) (OtherBodyIndex :type Integer) (bFromSweep :type Boolean) (SweepResult :type Hit%20Result%20Structure%20%28by%20ref%29))
  (Rendering|SetVisibility (Variables|Default|GetWidget) true false))

(event OnComponentEndOverlap(Sphere)
  (params (OverlappedComponent :type Primitive%20Component%20Object%20Reference) (OtherActor :type Actor%20Object%20Reference) (OtherComp :type Primitive%20Component%20Object%20Reference) (OtherBodyIndex :type Integer))
  (Rendering|SetVisibility (Variables|Default|GetWidget) false false))

(event Custom|Picked%20Up
  (Utilities|FlowControl|Delay 0.2)
  (Actor|DestroyActor))

(fn ConstructionScript
  (Utilities|FlowControl|Sequence
    (:then_0
      (if (Utilities|Enum|Equal(Enum) (Variables|Default|GetArmorPiece) "Pendant")
        (Components|StaticMesh|SetStaticMesh (Variables|Default|GetArmor) "/Game/Renea/Armor/HeartPendant.HeartPendant")))
    (:then_1
      (if (Utilities|Enum|Equal(Enum) (Variables|Default|GetArmorPiece) "Tiara")
        (Components|StaticMesh|SetStaticMesh (Variables|Default|GetArmor) "/Game/Renea/Armor/Tiara.Tiara")))
    (:then_2
      (if (Utilities|Enum|Equal(Enum) (Variables|Default|GetArmorPiece) "Bracelet")
        (Components|StaticMesh|SetStaticMesh (Variables|Default|GetArmor) "/Game/Renea/Armor/Bracelet.Bracelet")))))

(fn Equip/PickUp
  (CallFunction|PickedUp)
  (return (Variables|Default|GetArmorPiece)))