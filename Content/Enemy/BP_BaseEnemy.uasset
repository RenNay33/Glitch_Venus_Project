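; Base enemy with Venus flytrap animations that roams, chases the Rogue player on sight, and can be killed.
; Recursive AI MoveTo calls drive random roaming and, once pawn sensing fires, a chase that pauses movement for a looping attack animation on arrival.
; AttackSphere overlap applies damage to the Rogue independently of the attack cycle.
; Incoming damage lowers clamped health with sound and hit animation, destroying the actor at zero.
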(event OnSeePawn(PawnSensing)
  (params (Pawn :type Pawn%20Object%20Reference))
  ;[1 0.5 0.5 0.5] Player has been seen!
  (Variables|Default|SetIsSeeingPlayer true)
  ;;[1 0.5 0.5 0.5] Calling Function
  (CallFunction|ChasePlayer))

(event OnComponentBeginOverlap(AttackSphere)
  (params (OverlappedComponent :type Primitive%20Component%20Object%20Reference) (OtherActor :type Actor%20Object%20Reference) (OtherComp :type Primitive%20Component%20Object%20Reference) (OtherBodyIndex :type Integer) (bFromSweep :type Boolean) (SweepResult :type Hit%20Result%20Structure%20%28by%20ref%29))
  ;[1 0.5 0.5 0.5] Can Damage Player
  (bind _asrogue (Utilities|Casting|CastToRogue OtherActor))
  (Game|Damage|ApplyDamage _asrogue 1.0 0 self))

(event Custom|Chase%20Player
  ;[1 0.5 0.5 0.5] Custom Function - Chases player
  (if (Variables|Default|GetIsSeeingPlayer)
    (AI|AIMoveTo self "0, 0, 0" (Variables|Default|GetAs%20Rogue) 1.9e+02 false
      (:OnSuccess
        (if (Variables|Default|GetCan%20Attack)
          (Variables|Default|SetCan%20Attack false)
          (Components|Animation|PlayAnimation (Variables|Character|GetMesh) "/Game/Enemy/Animations/VenusFlyTrapAttack_Enemy_Anim.VenusFlyTrapAttack_Enemy_Anim" true)
          (Pawn|Components|CharacterMovement|SetMovementMode (Variables|Character|GetCharacterMovement) "MOVE_None" 0)
          (Utilities|FlowControl|Delay 2.0)
          (Pawn|Components|CharacterMovement|SetMovementMode (Variables|Character|GetCharacterMovement) "MOVE_Walking" 0)
          (Variables|Default|SetCan%20Attack true)
          (CallFunction|ChasePlayer))))))

(event Custom|Roaming
  ;[1 0.5 0.5 0.5] Roaming Function - Custom
  (AI|AIMoveTo self (.RandomLocation (AI|Navigation|GetRandomReachablePointinRadius (Transformation|GetActorLocation) 5e+02 0 0)) 0 5.0 false
    (:OnSuccess
      (Utilities|FlowControl|Delay 1.0)
      (CallFunction|Roaming))))

(event EventBeginPlay
  ;[1 0.5 0.5 0.5] Enemies are Roaming
  (CallFunction|Roaming))

(event Game|Damage|EventAnyDamage
  (params (Damage :type Float%20%28single-precision%29) (DamageType :type Damage%20Type%20Object%20Reference) (InstigatedBy :type Controller%20Object%20Reference) (DamageCauser :type Actor%20Object%20Reference))
  (bind _returnvalue (Transformation|GetActorLocation))
  ;[1 0.5 0.5 0.5] Enemy HP and Damage System
  (bind _output_get (Variables|Default|SetHealth (Math|Float|Clamp(Float) (- (Variables|Default|GetHealth) Damage) 0.0 5.0)))
  (if (== _output_get 0.0)
    (Audio|PlaySoundatLocation "/Game/Nadja/394466__plasterbrain__enemy-destroyed.394466__plasterbrain__enemy-destroyed" _returnvalue "0, 0, 0" 1.0 1.0 0.0 0 0 0 0)
    (Components|Animation|PlayAnimation (Variables|Character|GetMesh) "/Game/Enemy/Animations/VenusFlyTrapHit_Enemy_Anim.VenusFlyTrapHit_Enemy_Anim" false)
    (Actor|DestroyActor)
    (else
      (Audio|PlaySoundatLocation "/Engine/EditorSounds/Notifications/CompileFailed.CompileFailed" _returnvalue "0, 0, 0" 1.0 1.0 0.0 0 0 0 0)
      (Components|Animation|PlayAnimation (Variables|Character|GetMesh) "/Game/Enemy/Animations/VenusFlyTrapHit_Enemy_Anim.VenusFlyTrapHit_Enemy_Anim" false))))

(event EventTick
  (params (DeltaSeconds :type Float%20%28single-precision%29))
  ;[1 0.5 0.5 0.5] Making Player a Variable
  (bind _asrogue (Utilities|Casting|CastToRogue (Game|GetPlayerCharacter 0)))
  (Variables|Default|SetAs%20Rogue _asrogue))

(fn ConstructionScript)